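; BP_Obsticle2 is a breakable obstacle that teaches the heavy attack through an on-screen hint.
; On BeginPlay it sets the text of its WBP_Hint widget component to a hold-and-release LMB prompt.
; AnyDamage hides the Trunk, disables its collision and hides the hint only when a single hit's damage exceeds a fixed threshold; weaker hits just print a debug message.
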(event `self.ReceiveBeginPlay`
  (bind _aswbp_hint (cast `/Game/WaveGame/WaveCharacter/UI/WBP_Hint` (`WidgetComponent.GetWidget` (`self.Widget`))))
  (set `TextBlock.Text` "Hold LMB and release to heavy Attack" (`/Game/WaveGame/WaveCharacter/UI/WBP_Hint.Hint` _aswbp_hint)))

(event `self.ReceiveAnyDamage`
  (params (Damage :type "Float (single-precision)") (DamageType :type "DamageType Object Reference") (InstigatedBy :type "Controller Object Reference") (DamageCauser :type "Actor Object Reference"))
  (bind _trunk (`self.Trunk`))
  (`KismetSystemLibrary.PrintString` "Ayayayaya")
  (if (> Damage 10.0)
    (`SceneComponent.SetHiddenInGame` _trunk true false)
    (`PrimitiveComponent.SetCollisionEnabled` _trunk "NoCollision")
    (`SceneComponent.SetHiddenInGame` (`self.Widget`) true false)
    (else
      (`KismetSystemLibrary.PrintString` "TooWeek"))))

(fn `UserConstructionScript`)