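; BP_TreeBridge is a tree actor that falls over when it takes any damage, presumably to form a bridge.
; AnyDamage calls FallDown, which uses the Felt flag to run only once.
; FallDown snaps the Bridge component to a fallen pose using a fixed world-space offset and added roll, with no animation or sweep.
; It then fires the OnTreeDamaged dispatcher.
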(event `self.ReceiveBeginPlay`)

(event `FallDown`
  (bind _returnvalue (`SceneComponent.K2_GetComponentToWorld` (`self.Bridge`)))
  (if (not (`self.bFelt`))
    (set `self.bFelt` true)
    (bind _output_get (set `self.TargetTransform` (`KismetMathLibrary.MakeTransform` (+ (.location _returnvalue) (0.0 120.0 -180.0)) (`KismetMathLibrary.MakeRotator` (+ (.roll (.rotation _returnvalue)) 110.0) (.pitch (.rotation _returnvalue)) (.yaw (.rotation _returnvalue))) (.scale _returnvalue))))
    (`SceneComponent.K2_SetWorldTransform` (`self.Bridge`) _output_get false false)
    (`self.OnTreeDamaged`)))

(event `self.ReceiveAnyDamage`
  (params (Damage :type "Float (single-precision)") (DamageType :type "DamageType Object Reference") (InstigatedBy :type "Controller Object Reference") (DamageCauser :type "Actor Object Reference"))
  (`self.FallDown`))

(fn `UserConstructionScript`)