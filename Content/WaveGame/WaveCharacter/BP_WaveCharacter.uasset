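; Player character for the wave game, with sword and crossbow abilities, a charge-based dash and health.
; Controller ability signals pass an AC Abilities component readiness check, then drive light/heavy sword montages or charged crossbow projectiles.
; Sword damage uses timer-driven blade socket traces with a per-swing character ignore list.
; Dash walks capsule checks back from maximum range to a grounded, unblocked spot, lerps there by timeline and recharges on a timer.
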(event `SwordAttack`
  (params (InputState :type "/Game/WaveGame/WaveCharacter/CombatSystem/E_InputState Enum" :default "NewEnumerator0"))
  (bind _returnvalue (`self.GetActorForwardVector`))
  (bind _returnvalue_2 (`self.GetActorForwardVector`))
  (bind _value (`BlueprintMapLibrary.Map_Find` (`self.Abilities`) "NewEnumerator0"))
  (bind _returnvalue_3 (+ (+ (`self.K2_GetActorLocation`) (0.0 0.0 30.0)) (* _returnvalue 70.0)))
  (bind _returnvalue_4 (+ (+ (`self.K2_GetActorLocation`) (0.0 0.0 30.0)) (* _returnvalue_2 50.0)))
  (bind _extramontage (`/Game/WaveGame/WaveCharacter/CombatSystem/PDA_Ability.ExtraMontage` _value))
  ;[1 1 1 0.5] Sword
  ;;[0.2988 1 0.03321 0.5] Sword Attack Logic
  (switch `/Game/WaveGame/WaveCharacter/CombatSystem/E_InputState` InputState
    (:`NewEnumerator0`
      (`/Engine/EditorBlueprintResources/StandardMacros.IsValid` _value
        (:`Is Valid`
          (if (not (`BlueprintMapLibrary.Map_Find` (`self.isAbilityStarted`) "NewEnumerator0"))
            (`|PlayMontage` (`self.Mesh`) (`/Game/WaveGame/WaveCharacter/CombatSystem/PDA_Ability.StartMontage` _value) 1.0 0.0 "Started" false
              (:`then`
                (`BlueprintMapLibrary.Map_Add` (`self.isAbilityStarted`) "NewEnumerator0" true))
              (:`OnInterrupted`
                (`BlueprintMapLibrary.Map_Add` (`self.isAbilityStarted`) "NewEnumerator0")))))))
    (:`NewEnumerator1`
      (if (`BlueprintMapLibrary.Map_Find` (`self.isAbilityStarted`) "NewEnumerator0")
        (set `self.bIsSwordHeavyAttack` false)
        (`|PlayMontage` (`self.Mesh`) _extramontage 1.0 0.0 "Canceled"
          (:`then`
            (`GameplayStatics.PlaySound2D` "/Game/WaveGame/Sounds/Assets/sword_swoosh.sword_swoosh" 1.0 1.0 0.0 null null)
            (`BlueprintMapLibrary.Map_Add` (`self.isAbilityStarted`) "NewEnumerator0")
            (`KismetSystemLibrary.SphereTraceSingle` :`Start` _returnvalue_4 :`End` (+ _returnvalue_4 (* _returnvalue_2 100.0)) :`Radius` 50.0 :`TraceChannel` "TraceTypeQuery1" :`TraceColor` (struct :`G` 0.676039 :`B` 1.0 :`A` 1.0))
            (`/Game/WaveGame/WaveCharacter/CombatSystem/AC_AbilitiesComponent.UseAbility` (`self.AC_AbilitiesComponent`) "NewEnumerator0" :!label _label))
          (:`OnNotifyBegin`
            (`KismetSystemLibrary.PrintString` "Start"))
          (:`OnNotifyEnd`
            (`KismetSystemLibrary.PrintString` "End")))))
    (:`NewEnumerator2`
      (if (`BlueprintMapLibrary.Map_Find` (`self.isAbilityStarted`) "NewEnumerator0")
        (set `self.bIsSwordHeavyAttack` true)
        (`|PlayMontage` (`self.Mesh`) _extramontage 1.0 0.0 "Finished"
          (:`then`
            (`GameplayStatics.PlaySound2D` "/Game/WaveGame/Sounds/Assets/sword_swoosh.sword_swoosh" 1.0 1.0 0.0 null null)
            (`BlueprintMapLibrary.Map_Add` (`self.isAbilityStarted`) "NewEnumerator0")
            (`KismetSystemLibrary.SphereTraceSingle` :`Start` _returnvalue_3 :`End` (+ _returnvalue_3 (* _returnvalue (0.0 0.0 0.0))) :`Radius` 120.0 :`TraceChannel` "TraceTypeQuery1" :`TraceColor` (struct :`G` 0.019237 :`B` 1.0 :`A` 1.0))
            (goto _label)))))))

(event `self.ReceiveBeginPlay`
  (bind _asbp_wave_controller (cast `/Game/WaveGame/WaveCharacter/BP_WaveController` (`self.GetController`))) ; Кастим контроллер к нашему контроллеру
  (add `/Game/WaveGame/WaveCharacter/BP_WaveController.OnHandleAbility` _asbp_wave_controller (delegate `HandleAbility`)) ; Тут мы подписываемся на сигнал контроллера и указываем ивент, который отработает при получении сигнала
  (`self.SetSwordEffect`))

(event `HandleAbility`
  (params (State :type "/Game/WaveGame/WaveCharacter/CombatSystem/E_InputState Enum" :default "NewEnumerator0") (Ability :type "/Game/WaveGame/WaveCharacter/CombatSystem/E_Ability Enum" :default "NewEnumerator0"))
  ; Тут происходит обработка данных сигнала. Вызывается написанный мной метод (Даблклик на ExecuteAbility)
  (bind _isready (`/Game/WaveGame/WaveCharacter/CombatSystem/AC_AbilitiesComponent.CheckAbilityReady` (`self.AC_AbilitiesComponent`) Ability))
  (if _isready
    (switch `/Game/WaveGame/WaveCharacter/CombatSystem/E_Ability` Ability
      (:`NewEnumerator0`
        (`self.SwordAttack` State))
      (:`NewEnumerator1`
        (`self.ExecuteCrossbowAbility` State)))))

(event `self.ReceiveTick`
  (params (DeltaSeconds :type "Float (single-precision)")))

(event `DashBegin`
  (`self.CanDash`
    (:`Yes`
      (set `self.bIsDashing` true)
      (bind _result (`/Engine/EditorBlueprintResources/StandardMacros.DecrementInt` (`self.AvailableDashCount`))
        (:`  `
          (`self.OnDashChargesUpdated` _result)
          (if (not (`self.bIsDashRecharging`))
            (`self.DashCooldownBegin`))
          (set `self.AnimBlendValue` 0.0)
          (`|PlayMontage` (`self.Mesh`) "/Game/WaveGame/WaveCharacter/CharacterAssets/Anims/AM_Dash.AM_Dash" (/ 1.0 (`self.DashDuration`) (`self.AdditionalAnimDashScale`)) 0.0 "None" false
            (:`then`
              (`self.MoveOverTime` (`self.GetDashDestination` (`self.K2_GetActorLocation`) (`self.CalculateDashTargetLocation`))))
            (:`OnCompleted`
              (set `self.bIsDashing` false :!label _label_2))
            (:`OnInterrupted`
              (goto _label_2))))))))

(event `MoveOverTime`
  (params (Location :type "Vector Structure"))
  (bind _output_get (set `self.DashStartLocation` (`self.K2_GetActorLocation`)))
  (`self.K2_SetActorRotation` (`KismetMathLibrary.FindLookAtRotation` _output_get Location))
  (`TimelineComponent.SetPlayRate` (`self.DashTimeline`) (/ 1.0 (`self.DashDuration`)))
  (bind (_direction _locationalpha) (`Timeline|DashTimeline` :!via `PlayFromStart`)
    (:`Update`
      (`self.K2_SetActorLocation` (`KismetMathLibrary.VLerp` (`self.DashStartLocation`) Location _locationalpha)))))

(event `TriggerSwordCollision`
  ;[1 1 1 0.5] Sword
  ;;[0.15 0 0.01302 0.5] Sword Attack Collision Logic
  (bind _returnvalue (`KismetSystemLibrary.K2_SetTimerDelegate` (delegate `SwordLineTrace`) 0.02 true))
  (set `self.TriggetSwordEvent` _returnvalue))

(event `SwordLineTrace`
  ;[1 1 1 0.5] Sword
  ;;[0.15 0 0.01302 0.5] Sword Attack Collision Logic
  (bind (_outhit _returnvalue) (`KismetSystemLibrary.LineTraceSingle` :`Start` (`SceneComponent.GetSocketLocation` (`self.Sword`) "blade_start") :`End` (`SceneComponent.GetSocketLocation` (`self.Sword`) "blade_end") :`TraceChannel` "TraceTypeQuery1" :`TraceColor` (struct :`R` 0.006049 :`G` 1.0 :`B` 0.011232 :`A` 1.0)))
  (if _returnvalue
    (bind (_bblockinghit _binitialoverlap _time _distance _location _impactpoint _normal _impactnormal _physmat _hitactor) (`GameplayStatics.BreakHitResult` _outhit))
    (bind _ascharacter (cast `Character` _hitactor)
      (:`then`
        (if (== (`KismetArrayLibrary.Array_Find` (`self.ActorToIgnorDuringCurrentHit`) _hitactor) -1)
          (if (`self.bIsSwordHeavyAttack`)
            (`GameplayStatics.ApplyDamage` _ascharacter (* (`self.SwordDamage`) 4.0))
            (else
              (`GameplayStatics.ApplyDamage` _ascharacter (`self.SwordDamage`))))
          (`KismetArrayLibrary.Array_Add` (`self.ActorToIgnorDuringCurrentHit`) _ascharacter)))
      (:`CastFailed`
        (bind _asbp_obsticle (cast `/Game/WaveGame/Levels/Blueprints/BP_Obsticle` _hitactor))
        (`GameplayStatics.ApplyDamage` _asbp_obsticle (`self.SwordDamage`))))))

(event `DashCooldownBegin`
  (bind _returnvalue (`KismetSystemLibrary.K2_SetTimerDelegate` (delegate `ResetDashCount`) (`self.DashCooldownTime`) true))
  (set `self.bIsDashRecharging` true))

(event `ResetDashCount`
  (bind _result (`/Engine/EditorBlueprintResources/StandardMacros.IncrementInt` (`self.AvailableDashCount`))
    (:`  `
      (`self.OnDashChargesUpdated` _result)
      (if (== (`self.AvailableDashCount`) (`self.MaxDashCount`))
        (set `self.bIsDashRecharging` false)
        (`KismetSystemLibrary.K2_ClearAndInvalidateTimerHandle` (stale `DashCooldownBegin` _returnvalue))))))

(event `StopSwordCollision`
  ;[1 1 1 0.5] Sword
  ;;[0.15 0 0.01302 0.5] Sword Attack Collision Logic
  (`KismetSystemLibrary.K2_ClearAndInvalidateTimerHandle` (`self.TriggetSwordEvent`))
  (`KismetArrayLibrary.Array_Clear` (`self.ActorToIgnorDuringCurrentHit`)))

(event `TestEvent`)

(event `self.ReceiveAnyDamage`
  (params (Damage :type "Float (single-precision)") (DamageType :type "DamageType Object Reference") (InstigatedBy :type "Controller Object Reference") (DamageCauser :type "Actor Object Reference"))
  (`self.ChangeHP` (- (`self.CurrentHealth`) Damage)))

(event `EquipSword`
  (`SceneComponent.K2_AttachToComponent` (`self.Sword`) (`self.Mesh`) "HandSwordSocket" "KeepRelative" "KeepRelative" "KeepRelative" true))

(event `UnequipSword`
  (`SceneComponent.K2_AttachToComponent` (`self.Sword`) (`self.Mesh`) "BeltSwordSocket" "KeepRelative" "KeepRelative" "KeepRelative" true))

(event `StopAiming`
  (`|PlayMontage` (`self.Mesh`) (`/Game/WaveGame/WaveCharacter/CombatSystem/PDA_Ability.StartMontage` (`BlueprintMapLibrary.Map_Find` (`self.Abilities`) "NewEnumerator1")) 1.0 0.0 "Complited"
    (:`OnCompleted`
      _)
    (:`OnInterrupted`
      _)
    (:`OnNotifyEnd`
      _))
  (`self.UnequipCrossbow`)
  (`self.EquipSword`))

(event `EquipCrossbow`
  (`SceneComponent.K2_AttachToComponent` (`self.SM_CrossBow`) (`self.Mesh`) "HandCrossbowSocket" "KeepRelative" "KeepRelative" "KeepRelative" true))

(event `UnequipCrossbow`
  (`SceneComponent.K2_AttachToComponent` (`self.SM_CrossBow`) (`self.Mesh`) "BackCrossbowSocket" "KeepRelative" "KeepRelative" "KeepRelative" true)
  (`self.SetAttackRestriction` false true false true)
  (set `self.AnimBlendValue` 1.0))

(fn `CalculateDashTargetLocation`
  (returns (Location :type "Vector Structure"))
  (locals (TempMoveDir :type "Vector Structure"))
  (bind _returnvalue (`KismetMathLibrary.Normal` (`self.MovementDirection`)))
  (`KismetSystemLibrary.PrintString` (`KismetStringLibrary.Conv_VectorToString` _returnvalue))
  (return (+ (* (`KismetMathLibrary.SelectVector` (`self.GetActorForwardVector`) _returnvalue (== _returnvalue (0.0 0.0 0.0))) (`self.DashRange`)) (`self.K2_GetActorLocation`))))

(fn `ChangeHP`
  (params (DeltaValue :type "Float (double-precision)"))
  (bind _output_get (set `self.CurrentHealth` (`KismetMathLibrary.FClamp` (+ DeltaValue (`self.CurrentHealth`)) 0.0 (`self.MaxHealth`))))
  (`self.OnHealthUpdated` _output_get))

(fn `ExecuteCrossbowAbility`
  (params (InputState :type "/Game/WaveGame/WaveCharacter/CombatSystem/E_InputState Enum" :default "NewEnumerator0"))
  (bind _value (`BlueprintMapLibrary.Map_Find` (`self.Abilities`) "NewEnumerator1"))
  (switch `/Game/WaveGame/WaveCharacter/CombatSystem/E_InputState` InputState
    (:`NewEnumerator0`
      (`/Engine/EditorBlueprintResources/StandardMacros.IsValid` _value
        (:`Is Valid`
          (`self.PlayAnimMontage` (`/Game/WaveGame/WaveCharacter/CombatSystem/PDA_Ability.StartMontage` _value) 1.0 "Started")
          (`BlueprintMapLibrary.Map_Add` (`self.isAbilityStarted`) "NewEnumerator1" true))))
    (:`NewEnumerator2`
      (if (`self.bShotCharged`)
        (`|SpawnActorFromClass` "/Game/WaveGame/WaveCharacter/Projectile/BP_Projectile.BP_Projectile_C" (`self.GetTransform` self) "Undefined" "MultiplyWithRoot" null null)
        (`BlueprintMapLibrary.Map_Add` (`self.isAbilityStarted`) "NewEnumerator1")
        (`/Game/WaveGame/WaveCharacter/CombatSystem/AC_AbilitiesComponent.UseAbility` (`self.AC_AbilitiesComponent`) "NewEnumerator1")
        (`self.SetChargeTime` 0.0)))
    (:`NewEnumerator4`
      (`KismetSystemLibrary.PrintString` (`KismetStringLibrary.Conv_DoubleToString` (`self.ShootChargeTime`))))))

(fn `ExecuteSwordAbility`
  (params (InputState :type "/Game/WaveGame/WaveCharacter/CombatSystem/E_InputState Enum" :default "NewEnumerator0"))
  (bind _returnvalue (`self.GetActorForwardVector`))
  (bind _returnvalue_2 (`self.GetActorForwardVector`))
  (bind _value (`BlueprintMapLibrary.Map_Find` (`self.Abilities`) "NewEnumerator0"))
  (bind _returnvalue_3 (+ (+ (`self.K2_GetActorLocation`) (0.0 0.0 30.0)) (* _returnvalue 50.0)))
  (bind _returnvalue_4 (+ (+ (`self.K2_GetActorLocation`) (0.0 0.0 30.0)) (* _returnvalue_2 50.0)))
  (bind _startmontage (`/Game/WaveGame/WaveCharacter/CombatSystem/PDA_Ability.StartMontage` _value))
  (bind _extramontage (`/Game/WaveGame/WaveCharacter/CombatSystem/PDA_Ability.ExtraMontage` _value))
  (switch `/Game/WaveGame/WaveCharacter/CombatSystem/E_InputState` InputState
    (:`NewEnumerator0`
      (`/Engine/EditorBlueprintResources/StandardMacros.IsValid` _value
        (:`Is Valid`
          (`BlueprintMapLibrary.Map_Add` (`self.isAbilityStarted`) "NewEnumerator0" true)
          (`self.PlayAnimMontage` _startmontage 1.0 "Started"))))
    (:`NewEnumerator1`
      (`self.MoveAndTurnNotify` false)
      (`self.MoveAndTurnNotify` true)
      (`self.PlayAnimMontage` _extramontage 1.0 "Canceled")
      (`BlueprintMapLibrary.Map_Add` (`self.isAbilityStarted`) "NewEnumerator0")
      (`KismetSystemLibrary.SphereTraceSingle` :`Start` _returnvalue_4 :`End` (+ _returnvalue_4 (* _returnvalue_2 100.0)) :`Radius` 60.0 :`TraceChannel` "TraceTypeQuery1" :`TraceColor` (struct :`G` 0.676039 :`B` 1.0 :`A` 1.0))
      (`/Game/WaveGame/WaveCharacter/CombatSystem/AC_AbilitiesComponent.UseAbility` (`self.AC_AbilitiesComponent`) "NewEnumerator0" :!label _label))
    (:`NewEnumerator2`
      (if (`BlueprintMapLibrary.Map_Find` (`self.isAbilityStarted`) "NewEnumerator0")
        (`self.MoveAndTurnNotify` false)
        (`self.MoveAndTurnNotify` true)
        (`self.PlayAnimMontage` _extramontage 1.0 "Finished")
        (`BlueprintMapLibrary.Map_Add` (`self.isAbilityStarted`) "NewEnumerator0")
        (`KismetSystemLibrary.SphereTraceSingle` :`Start` _returnvalue_3 :`End` (+ _returnvalue_3 (* _returnvalue 150.0)) :`Radius` 120.0 :`TraceChannel` "TraceTypeQuery1" :`DrawDebugType` "ForDuration" :`TraceColor` (struct :`G` 0.019237 :`B` 1.0 :`A` 1.0))
        (goto _label)))
    (:`NewEnumerator4`
      (`self.PlayAnimMontage` _startmontage 1.0 "Ongoing"))))

(fn `GetDashDestination`
  (params (Start :type "Vector Structure") (End :type "Vector Structure"))
  (returns (Location :type "Vector Structure"))
  (locals (Direction :type "Vector Structure" :default (0.0 0.0 0.0)) (CapsuleDiameter :type "Float (double-precision)") (CapsuleCount :type Integer) (CurrentCapsuleLocation :type "Vector Structure"))
  (bind (_outradius _outhalfheight) (`CapsuleComponent.GetUnscaledCapsuleSize` (`self.CapsuleComponent`)))
  (set `local.Direction` (`KismetMathLibrary.GetDirectionUnitVector` Start End))
  (bind _output_get (set `local.CapsuleDiameter` (* (`CapsuleComponent.CapsuleRadius` (`self.CapsuleComponent`)) 2.0)))
  (bind _output_get_2 (set `local.CapsuleCount` (/ (`KismetMathLibrary.Vector_Distance` Start End) _output_get)))
  (for _index (range (+ _output_get_2 1))
    (bind _output_get_3 (set `local.CurrentCapsuleLocation` (+ (* (- (`local.CapsuleCount`) _index) (`local.Direction`) (`local.CapsuleDiameter`)) (`local.Start`))))
    (bind _outhits (`KismetSystemLibrary.CapsuleTraceMultiForObjects` :`Start` _output_get_3 :`End` _output_get_3 :`Radius` _outradius :`HalfHeight` _outhalfheight :`ObjectTypes` (`|MakeArray` "ObjectTypeQuery1" "ObjectTypeQuery2" "ObjectTypeQuery3" "ObjectTypeQuery5" "ObjectTypeQuery6" :!type "EObjectTypeQuery Enum") :`DrawDebugType` "ForDuration"))
    (bind _bisvalid (`self.IsValidDashLocation` (`local.CurrentCapsuleLocation`) _outhits))
    (if _bisvalid
      (return (`local.CurrentCapsuleLocation`))))
  (return (`local.Start`)))

(fn `IsValidDashLocation`
  (params (Location :type "Vector Structure") (Hits :type "Array of HitResult Structure"))
  (returns (bIsValid :type Boolean))
  (bind _hits (`local.Hits`))
  (bind (_outhit _returnvalue) (`KismetSystemLibrary.LineTraceSingle` Location (- Location (0.0 0.0 500.0)) "TraceTypeQuery1"))
  (if _returnvalue
    (if (`KismetArrayLibrary.Array_IsEmpty` _hits)
      (return true)
      (else
        (for _array_element _hits
          (if (`|EnumEquality` (`PrimitiveComponent.GetCollisionResponseToChannel` (`.HitComponent` (`GameplayStatics.BreakHitResult` _array_element)) "ECC_WorldStatic") "ECR_Block")
            (return false)))
        (return true)))
    (else
      (return false))))

(fn `SetAttackRestriction`
  (params (bTurnUpdate :type Boolean) (bMoveUpdate :type Boolean) (NewTurnValue :type Boolean) (NewMoveValue :type Boolean))
  (if bTurnUpdate
    (`self.MoveAndTurnNotify` true NewTurnValue))
  (if bMoveUpdate
    (`self.MoveAndTurnNotify` false NewMoveValue)))

(fn `SetChargeTime`
  (params (Time :type "Float (double-precision)"))
  (bind _output_get (set `self.ShootChargeTime` Time))
  (set `self.bShotCharged` (>= _output_get (`self.AimingTime`))))

(fn `SetSwordEffect`
  (bind _sword (`self.Sword`))
  (bind _returnvalue (`SceneComponent.GetSocketLocation` _sword "Blade_Start"))
  (bind _returnvalue_2 (`SceneComponent.GetSocketLocation` _sword "Blade_end"))
  (bind _returnvalue_3 (- _returnvalue _returnvalue_2))
  (bind _returnvalue_4 (`NiagaraFunctionLibrary.SpawnSystemAttached` "/Game/WaveGame/WaveCharacter/CharacterAssets/Effects/NS_Sword.NS_Sword" _sword "None" (/ (+ _returnvalue _returnvalue_2) 2) (`KismetMathLibrary.MakeRotFromZ` _returnvalue_3) "KeepWorldPosition"))
  (`FXSystemComponent.SetFloatParameter` _returnvalue_4 "TrailWidth" (`KismetMathLibrary.VSize` _returnvalue_3))
  (bind _output_get (set `self.SwordTrailEffect` _returnvalue_4))
  (`ActorComponent.Deactivate` _output_get))

(fn `UserConstructionScript`
  (set `self.AvailableDashCount` (`self.MaxDashCount`)))