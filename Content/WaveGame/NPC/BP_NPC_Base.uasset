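; Base NPC Blueprint that shows a timed, state-dependent dialogue line in a widget when something overlaps its interaction trigger.
; StartDialogue looks up the current state's line, displays it on DialoguePrompt and sets a timer for EndDialogue, which hides it and advances the state from Idle through Busy to Minor.
; On BeginPlay it binds to every BP_Trigger's signal.
; GetNPCState always returns Idle, and the player-cast interaction logic is disconnected.
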(event `self.ReceiveBeginPlay`
  (bind _outactors (`GameplayStatics.GetAllActorsOfClass` "/Game/WaveGame/NPC/BP_Trigger.BP_Trigger_C"))
  (for _array_element _outactors
    (`self.BindToStateChanger` _array_element)))

(event `self.InteractionTrigger.OnComponentBeginOverlap`
  (params (OverlappedComponent :type "PrimitiveComponent Object Reference") (OtherActor :type "Actor Object Reference") (OtherComp :type "PrimitiveComponent Object Reference") (OtherBodyIndex :type Integer) (bFromSweep :type Boolean) (SweepResult :type "HitResult Structure (by ref)"))
  (`self.StartDialogue`))

(event `self.InteractionTrigger.OnComponentEndOverlap`
  (params (OverlappedComponent :type "PrimitiveComponent Object Reference") (OtherActor :type "Actor Object Reference") (OtherComp :type "PrimitiveComponent Object Reference") (OtherBodyIndex :type Integer)))

(fn `AdvanceState`
  (switch `/Game/WaveGame/NPC/E_NPC_State` (`self.CurrentState`)
    (:`NewEnumerator0`
      (`self.SetNPCState ` "NewEnumerator1"))
    (:`NewEnumerator1`
      (`self.SetNPCState ` "NewEnumerator4"))))

(fn `BindToStateChanger`
  (params (Trigger :type "/Game/WaveGame/NPC/BP_Trigger Object Reference"))
  (add `/Game/WaveGame/NPC/BP_Trigger.Signal` Trigger (`|CreateDelegate` :!event `SetNPCState `)))

(fn `EndDialogue`
  (set `self.bIsSpeaking` false)
  (`SceneComponent.SetVisibility` (`self.DialoguePrompt`) false false)
  (`self.AdvanceState`))

(fn `GetNPCState`
  (returns (currentState :type "/Game/WaveGame/NPC/E_NPC_State Enum"))
  (return "NewEnumerator0"))

(fn `SetNPCState `
  (params (NewState :type "/Game/WaveGame/NPC/E_NPC_State Enum" :default "NewEnumerator0"))
  (bind _output_get (set `self.CurrentState` NewState))
  (`self.OnStateChanged ` _output_get))

(fn `StartDialogue`
  (bind _dialogueprompt (`self.DialoguePrompt`))
  (bind (_value _returnvalue) (`BlueprintMapLibrary.Map_Find` (`self.DialogueLinesMap `) (`self.CurrentState`)))
  (`self.bIsSpeaking`
    (:`then`
      (`KismetSystemLibrary.PrintString` "Already speaking"))
    (:`else`
      (set `self.bIsSpeaking` true)
      (if _returnvalue
        (set `self.CurrentDialogue` _value)
        (bind _aswbp_dialogue (cast `/Game/WaveGame/NPC/WBP_Dialogue` (`WidgetComponent.GetWidget` _dialogueprompt)))
        (`/Game/WaveGame/NPC/WBP_Dialogue.SetDialogueText` _aswbp_dialogue (`KismetTextLibrary.Conv_StringToText` (`self.CurrentDialogue`)))
        (`SceneComponent.SetVisibility` _dialogueprompt true false)
        (`KismetSystemLibrary.K2_SetTimer` null "EndDialogue" 3.0)
        (else
          (set `self.CurrentDialogue` "БЛЯЯЯЯЯЯЯЯЯЯЯ ОНО СЛОМАЛОСЬ"))))))

(fn `UserConstructionScript`)