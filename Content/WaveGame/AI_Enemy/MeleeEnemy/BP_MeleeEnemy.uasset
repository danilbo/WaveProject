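; BP_MeleeEnemy is a melee AI enemy in WaveGame that bites the player and ragdolls on death before being destroyed.
; Taking damage or an AlertOthers call writes the target and alert flag to its Blackboard, and death stops the AI's brain logic.
; Attack plays a bite montage whose notify fires a short forward sphere trace to damage BP_WaveCharacter, then signals attack end.
; NotifyGroup is an empty stub.
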(event `self.ReceiveTick`
  (params (DeltaSeconds :type "Float (single-precision)")))

(event `self.ReceiveBeginPlay`
  (set `self.CurrentHealth` (`self.MaxHealth`)))

(event `self.ReceiveAnyDamage`
  (params (Damage :type "Float (single-precision)") (DamageType :type "DamageType Object Reference") (InstigatedBy :type "Controller Object Reference") (DamageCauser :type "Actor Object Reference"))
  (bind _returnvalue (`AIBlueprintHelperLibrary.GetBlackboard` (`AIBlueprintHelperLibrary.GetAIController` self)))
  (bind _output_get (set `self.CurrentHealth` (- (`self.CurrentHealth`) Damage)))
  (if (<= _output_get 0.0)
    (`self.Die`)
    (else
      (`BlackboardComponent.SetValueAsObject` _returnvalue (`self.TargetActor`) DamageCauser)
      (`BlackboardComponent.SetValueAsBool` _returnvalue (`self.IsAlerted`) true))))

(event `Die`
  (`BrainComponent.StopLogic` (`AIController.BrainComponent` (`AIBlueprintHelperLibrary.GetAIController` self)) "Dead")
  (`CharacterMovementComponent.DisableMovement` (`self.CharacterMovement`))
  (`PrimitiveComponent.SetCollisionEnabled` (`self.CapsuleComponent`) "NoCollision")
  (`PrimitiveComponent.SetSimulatePhysics` (`self.Mesh`) true)
  (`KismetSystemLibrary.Delay` 10.0)
  (`self.K2_DestroyActor`))

(event `Attack`
  (bind _returnvalue (`self.K2_GetActorLocation`))
  (`|PlayMontage` (`self.Mesh`) "/Game/WaveGame/Enemies/Dog/AM_DogBIteNew.AM_DogBIteNew"
    (:`OnCompleted`
      (`self.OnAttackEnd`))
    (:`OnInterrupted`
      (`self.OnAttackEnd`))
    (:`OnNotifyBegin`
      (bind (_outhit _returnvalue_2) (`KismetSystemLibrary.SphereTraceSingle` :`Start` _returnvalue :`End` (+ _returnvalue (* (`KismetMathLibrary.GetForwardVector` (`self.K2_GetActorRotation`)) 150.0)) :`Radius` 5.0 :`TraceChannel` "TraceTypeQuery1" :`DrawDebugType` "ForDuration"))
      (if _returnvalue_2
        (`GameplayStatics.ApplyDamage` (cast `/Game/WaveGame/WaveCharacter/BP_WaveCharacter` (`.HitActor` (`GameplayStatics.BreakHitResult` _outhit)) :!pure true) (`self.AttackDamage`))
        (`self.OnAttackEnd`)))))

(event `/Game/WaveGame/AI_Enemy/MeleeEnemy/BPI_EnemyGroup.AlertOthers`
  (params (NewTarget :type "Actor Object Reference"))
  (bind _returnvalue (`AIBlueprintHelperLibrary.GetBlackboard` (`AIBlueprintHelperLibrary.GetAIController` self)))
  (`BlackboardComponent.SetValueAsObject` _returnvalue (`self.TargetActor`) NewTarget)
  (`BlackboardComponent.SetValueAsBool` _returnvalue (`self.IsAlerted`) true)
  (set `self.Is Alerted` true))

(fn `NotifyGroup`
  (params (FoundTarget :type "Actor Object Reference")))

(fn `UserConstructionScript`)