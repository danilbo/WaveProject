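; BP_RangeEnemy is an AI ranged enemy with health, death and an arrow attack.
; Non-lethal damage sets the damage causer as the blackboard target and raises an alert.
; Death stops AI logic, disables movement and capsule collision, ragdolls the mesh, then destroys the actor after a delay.
; Attack plays a shot montage and spawns an arrow at the fire socket on completion, though its Attacking guard never engages.
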(event `self.ReceiveBeginPlay`
  (set `self.CurrentHealth` (`self.MaxHealth`)))

(event `self.ReceiveAnyDamage`
  (params (Damage :type "Float (single-precision)") (DamageType :type "DamageType Object Reference") (InstigatedBy :type "Controller Object Reference") (DamageCauser :type "Actor Object Reference"))
  (bind _returnvalue (`AIBlueprintHelperLibrary.GetBlackboard` (`AIBlueprintHelperLibrary.GetAIController` self)))
  (bind _output_get (set `self.CurrentHealth` (- (`self.CurrentHealth`) Damage)))
  (if (<= _output_get 0.0)
    (`self.Die`)
    (else
      (`BlackboardComponent.SetValueAsObject` _returnvalue (`self.TargetActor`) DamageCauser)
      (`BlackboardComponent.SetValueAsBool` _returnvalue (`self.IsAlerted`) true))))

(event `Die`
  (`BrainComponent.StopLogic` (`AIController.BrainComponent` (`AIBlueprintHelperLibrary.GetAIController` self)) "Dead")
  (`CharacterMovementComponent.DisableMovement` (`self.CharacterMovement`))
  (`PrimitiveComponent.SetCollisionEnabled` (`self.CapsuleComponent`) "NoCollision")
  (`PrimitiveComponent.SetSimulatePhysics` (`self.Mesh`) true)
  (`KismetSystemLibrary.Delay` 10.0)
  (`self.K2_DestroyActor`))

(event `Attack`
  (if (`self.Attacking`)
    (set `self.Attacking` true)
    (else
      (`|PlayMontage` (`self.Mesh`) "/Game/WaveGame/Enemies/Fairy/Anims/AM_FairyShot.AM_FairyShot"
        (:`OnCompleted`
          (`|SpawnActorFromClass` "/Game/WaveGame/AI_Enemy/RangeEnemy/BP_Arrow.BP_Arrow_C" (`SceneComponent.GetSocketTransform` (`self.StaticMesh`) "FireSocket" "RTS_World") "Undefined" "MultiplyWithRoot" null null)
          (set `self.Attacking` false))))))

(fn `UserConstructionScript`)