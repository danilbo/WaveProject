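; Sword attack ability Blueprint for the wave game's combat system, driven by ExecuteAbility states Started, Canceled and Finished.
; Each state plays the matching section of the ability montage on the owning character's mesh.
; Canceled and Finished also fire a forward sphere trace, wider on Finished, with persistent debug drawing.
; The traces test only the owner's own mesh component, and their results are unused, so no damage is applied here.
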(event `self.ExecuteAbility`
  (params (State :type "/Game/WaveGame/CombatSystem/E_InputState Enum" :default "NewEnumerator0"))
  (bind _ownercharacter (`self.GetOwnerCharacter`))
  (bind _ownercharacter_2 (`self.GetOwnerCharacter`))
  (bind (_returnvalue_x _returnvalue_y _returnvalue_z) (`KismetMathLibrary.BreakVector` (`Actor.K2_GetActorLocation` _ownercharacter)))
  (bind _returnvalue (`Actor.GetActorForwardVector` _ownercharacter))
  (bind (_returnvalue_x_2 _returnvalue_y_2 _returnvalue_z_2) (`KismetMathLibrary.BreakVector` (`Actor.K2_GetActorLocation` _ownercharacter_2)))
  (bind _returnvalue_2 (`Actor.GetActorForwardVector` _ownercharacter_2))
  (bind _returnvalue_3 (+ (`KismetMathLibrary.MakeVector` _returnvalue_x_2 _returnvalue_y_2 (+ _returnvalue_z_2 30.0)) (* _returnvalue_2 60.0)))
  (bind _returnvalue_4 (+ (`KismetMathLibrary.MakeVector` _returnvalue_x _returnvalue_y (+ _returnvalue_z 30.0)) (* _returnvalue 60.0)))
  (switch `/Game/WaveGame/CombatSystem/E_InputState` State
    (:`NewEnumerator0`
      (`|PlayMontage` (`Character.Mesh` (`self.GetOwnerCharacter`)) (`self.AbilityMontage`) 1.0 0.0 "Started"))
    (:`NewEnumerator1`
      (`|PlayMontage` (`Character.Mesh` (`self.GetOwnerCharacter`)) (`self.AbilityMontage`) 1.0 0.0 "Canceled"
        (:`then`
          (`PrimitiveComponent.K2_SphereTraceComponent` (`Character.Mesh` _ownercharacter_2) _returnvalue_3 (+ (* _returnvalue_2 500.0) _returnvalue_3) 60.0 true true true))))
    (:`NewEnumerator2`
      (`|PlayMontage` (`Character.Mesh` (`self.GetOwnerCharacter`)) (`self.AbilityMontage`) 1.0 0.0 "Finished"
        (:`then`
          (`PrimitiveComponent.K2_SphereTraceComponent` (`Character.Mesh` _ownercharacter) _returnvalue_4 (+ (* _returnvalue 500.0) _returnvalue_4) 120.0 true true true))))))